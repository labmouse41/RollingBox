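; BP_MainMenu_Controller is the main menu player controller, which sets up UI-only input with a visible cursor for the local player on BeginPlay.
; EndClientSession destroys the online session, then reopens the MainMenu level.
; UIShowLobbyMenu lazily creates, caches and displays the WB_LobbyMenu widget, but its call is unwired and the ShowLobbyMenu event is empty.
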(event `self.ReceiveBeginPlay`
  (if (`self.IsLocalController`)
    (set `self.bShowMouseCursor` true)
    (`WidgetBlueprintLibrary.SetInputMode_UIOnlyEx` self null)))

(event `EndClientSession`
  (`DestroySessionCallbackProxy.DestroySession` self
    (:`then`
      (`GameplayStatics.OpenLevel` "MainMenu"))))

(event `Show Lobby Menu`)

(fn `UI Show Lobby Menu`
  (`/Engine/EditorBlueprintResources/StandardMacros.IsValid` (`self.WB Lobby Menu`)
    (:`Is Valid`
      _)
    (:`Is Not Valid`
      (bind _returnvalue (`|CreateWidget` "/Game/Widget/WB_LobbyMenu.WB_LobbyMenu_C" (`GameplayStatics.GetPlayerController` 0)))
      (set `self.WB Lobby Menu` _returnvalue)))
  (`UserWidget.AddToViewport` (`self.WB Lobby Menu`) 0)
  (return))

(fn `UserConstructionScript`)