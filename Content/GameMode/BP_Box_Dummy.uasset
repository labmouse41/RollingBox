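; BP_Box_Dummy is a physics cube in a GameMode folder, apparently a stripped-down dummy of a jumping box.
; Tick clamps cube velocity to MaxSpeedByHit and accumulates AirTime while speed exceeds a threshold.
; Jump, CapMaxSpeed and nearest-point helpers are defined but uncalled here.
; Ground-trace check, beat-driven edge glow, touch particles and squared-distance helper have disconnected bodies, so they do nothing.
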(event `self.ReceiveTick`
  (params (DeltaSeconds :type "Float (single-precision)"))
  (bind _maxspeedbyhit (`self.MaxSpeedByHit`))
  ;[1 1 1] Tick
  (`|ExecutionSequence`
    (:`then_0`
      (`self.SetEdgeGlowColor`)
      (bind _returnvalue (`PrimitiveComponent.GetPhysicsLinearVelocity` (`self.Cube`) "None"))
      (if (> (`KismetMathLibrary.VSize` _returnvalue) _maxspeedbyhit)
        (`PrimitiveComponent.SetPhysicsLinearVelocity` (`self.Cube`) (* _maxspeedbyhit (`KismetMathLibrary.Normal` _returnvalue)) false "None")))
    (:`then_1`
      (bind _returnvalue_2 (`PrimitiveComponent.GetPhysicsLinearVelocity` (`self.Cube`) "None"))
      (if (> (`KismetMathLibrary.VSize` _returnvalue_2) 222.0)
        (set `self.AirTime` (+ DeltaSeconds (`self.AirTime`)))))))

(event `self.ReceiveBeginPlay`)

(fn `CapMaxSpeed`
  (bind _maxspeed (`self.MaxSpeed`))
  (bind _returnvalue (`PrimitiveComponent.GetPhysicsLinearVelocity` (`self.Cube`) "None"))
  (if (> (`KismetMathLibrary.VSize` _returnvalue) _maxspeed)
    (`PrimitiveComponent.SetPhysicsLinearVelocity` (`self.Cube`) (* _maxspeed (`KismetMathLibrary.Normal` _returnvalue)) false "None")))

(fn `CastLineToBottom`
  (params (OffSet :type "Vector Structure"))
  (returns (Detected :type Boolean))
  (bind (_outhit _returnvalue) (`KismetSystemLibrary.LineTraceSingleForObjects` OffSet (- OffSet (0.0 0.0 2.2)) (`|MakeArray` "ObjectTypeQuery1" "ObjectTypeQuery2" "ObjectTypeQuery3" "ObjectTypeQuery4" "ObjectTypeQuery5" "ObjectTypeQuery6" :!type "EObjectTypeQuery Enum") false (`self.Obstacles`) "None" true (struct :`R` 1.0 :`A` 1.0) (struct :`G` 1.0 :`A` 1.0) 1.0))
  (return _returnvalue))

(fn `GetLengthSquaredFromComponentToPoint`
  (params (InComponent :type "SceneComponent Object Reference") (point :type "Vector Structure"))
  (returns (LengthSquared :type "Float (double-precision)") (OutComponent :type "SceneComponent Object Reference")))

(fn `Jump`
  (bind (_returnvalue _touchingthis) (`self.OnGround?`))
  (if _returnvalue
    (bind _returnvalue_2 (`PrimitiveComponent.GetPhysicsLinearVelocity` (`self.Cube`) "None"))
    (`PrimitiveComponent.SetPhysicsLinearVelocity` (`self.Cube`) (`KismetMathLibrary.MakeVector` (.x _returnvalue_2) (.y _returnvalue_2) (`self.JumpForce`)) false "None")
    (`self.PlayJumpParticlesOnPoint` (`SceneComponent.RelativeLocation` _touchingthis) _touchingthis)))

(fn `OnGround?`
  (returns (ReturnValue :type Boolean) (TouchingThis :type "SceneComponent Object Reference"))
  (locals (TouchingThisOne :type "SceneComponent Object Reference")))

(fn `PlayJumpParticlesOnPoint`
  (params (PlayLocation :type "Vector Structure") (CheckVelocityHere :type "SceneComponent Object Reference"))
  (`SceneComponent.K2_SetRelativeLocation` (`self.NG_ParticleOnJump`) PlayLocation false false)
  (bind _returnvalue (`PrimitiveComponent.GetPhysicsLinearVelocityAtPoint` (`self.Cube`) (`SceneComponent.RelativeLocation` CheckVelocityHere) "None"))
  (`FXSystemComponent.SetVectorParameter` (`self.NG_ParticleOnJump`) "InheritVelocity" (* _returnvalue 0.01))
  (`NiagaraComponent.ResetSystem` (`self.NG_ParticleOnJump`))
  (set `self.AirTime` 0.0))

(fn `PlayTouchParticlesOnPoint`
  (params (PlayLocation :type "Vector Structure") (CheckVelocityHere :type "SceneComponent Object Reference")))

(fn `SetEdgeGlowColor`)

(fn `SetNearestPoint`
  (params (InComponent :type "SceneComponent Object Reference") (point :type "Vector Structure"))
  (bind (_lengthsquared _outcomponent) (`self.GetLengthSquaredFromComponentToPoint` InComponent point))
  (if (< _lengthsquared (`self.NearestLength`))
    (set `self.NearestLength` _lengthsquared)
    (set `self.NearestPointAmong8` _outcomponent)))

(fn `UserConstructionScript`)