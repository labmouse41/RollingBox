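; BP_MyGameMode is a game mode that acts as a rhythm clock, tracking whether the game is currently on the beat.
; Each Tick feeds game time and BeatLength into a cosine wave, then clamps it against OnBeatStrictHowMuch to form a window around each beat.
; When that state flips, it updates OnBeat and calls SetOnBeat, apparently an event dispatcher.
; While OnBeat is true, it prints a debug string.
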(event `self.ReceiveTick`
  (params (DeltaSeconds :type "Float (single-precision)"))
  (bind _returnvalue (!= (`KismetMathLibrary.MapRangeClamped` (`KismetMathLibrary.DegCos` (* (`self.GetGameTimeSinceCreation`) 360.0 (/ 1.0 (`self.BeatLength`)))) (`self.OnBeatStrictHowMuch`) 1.0 0.0 1.0) 0.0))
  (if (`self.bOnBeat`)
    (`KismetSystemLibrary.PrintString` "OnBeat" true true (struct :`G` 1.0 :`B` 0.345176 :`A` 1.0) 0.1))
  (if (!= (`self.bOnBeat`) _returnvalue)
    (set `self.bOnBeat` _returnvalue)
    (`self.EVDC_SetOnBeat`)))

(fn `UserConstructionScript`)