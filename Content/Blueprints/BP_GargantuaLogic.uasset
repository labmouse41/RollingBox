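; BP_GargantuaLogic is a black hole that pulls in BP_CBox actors and spits them out of another black hole.
; On BeginPlay the authority picks a random other instance as Exit.
; Outer overlap activates an inverse-square pull, added to box velocity each Tick without delta-time scaling.
; Center overlap teleports the box to Exit and launches it randomly upward, briefly disabling Exit's collision to prevent recapture; beat-synced variants are unused here.
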(event `self.ReceiveBeginPlay`
  ;[1 1 1] SetExit
  (`/Engine/EditorBlueprintResources/ActorMacros.Switch Has Authority`
    (:`Authority`
      (bind _outactors (`GameplayStatics.GetAllActorsOfClass` "BP_GargantuaLogic_C"))
      (bind _output_get (set `self.HoleList` _outactors))
      (`KismetArrayLibrary.Array_RemoveItem` _output_get self)
      (set `self.Exit` (`KismetArrayLibrary.Array_Random` (`self.HoleList`))))))

(event `self.ReceiveTick`
  (params (DeltaSeconds :type "Float (single-precision)"))
  ;[1 1 1] Gravity
  (if (`self.BlackHoleOn`)
    (for _array_element (`PrimitiveComponent.GetOverlappingActors` (`self.Outer`) "/Game/GameMode/BP_CBox.BP_CBox_C")
      (bind _asbp_cbox (cast `/Game/GameMode/BP_CBox` _array_element))
      (bind _returnvalue (- (`self.K2_GetActorLocation`) (`self.K2_GetActorLocation` _asbp_cbox)))
      (`PrimitiveComponent.SetPhysicsLinearVelocity` (`BoxCharacter.Cube` _asbp_cbox) (/ (* (`KismetMathLibrary.Normal` _returnvalue) (`self.Gravity`)) (`KismetMathLibrary.VSizeSquared` _returnvalue)) true "None"))))

(event `self.Center.OnComponentBeginOverlap`
  (params (OverlappedComponent :type "PrimitiveComponent Object Reference") (OtherActor :type "Actor Object Reference") (OtherComp :type "PrimitiveComponent Object Reference") (OtherBodyIndex :type Integer) (bFromSweep :type Boolean) (SweepResult :type "HitResult Structure (by ref)"))
  (if (not (`self.IsExit`))
    (bind _asbp_cbox (cast `/Game/GameMode/BP_CBox` OtherActor))
    (set `self.As BP CBox` _asbp_cbox)
    (`self.SetExit`)
    (`self.Release`)))

(event `self.Outer.OnComponentBeginOverlap`
  (params (OverlappedComponent :type "PrimitiveComponent Object Reference") (OtherActor :type "Actor Object Reference") (OtherComp :type "PrimitiveComponent Object Reference") (OtherBodyIndex :type Integer) (bFromSweep :type Boolean) (SweepResult :type "HitResult Structure (by ref)"))
  (set `self.BlackHoleOn` true))

(fn `Release`
  (bind (_returnvalue_x _returnvalue_y _returnvalue_z) (`KismetMathLibrary.BreakVector` (`KismetMathLibrary.RandomUnitVector`)))
  (bind _as_bp_cbox (`self.As BP CBox`))
  (`self.SetLocationToExit` (`self.As BP CBox`) (`self.Exit`))
  (`PrimitiveComponent.SetPhysicsLinearVelocity` (`BoxCharacter.Cube` _as_bp_cbox) (* (+ (`KismetMathLibrary.MakeVector` _returnvalue_x _returnvalue_y (`KismetMathLibrary.Abs` _returnvalue_z)) (0.0 0.0 1.0)) (`self.OutPower`)) false "None")
  (`BoxCharacter.SetAirTime` _as_bp_cbox 0.0)
  (set `self.BlackHoleOn` false)
  (`KismetSystemLibrary.K2_SetTimer` null "ResetExit" 0.2))

(fn `ReleaseOnBeat`
  (if (`/Game/Blueprints/BeatChecker.bOnBeat` (`self.BeatChecker`))
    (`self.Release`)
    (else
      (`KismetSystemLibrary.K2_SetTimer` null "ReleaseOnBeat" 0.05))))

(fn `ResetEffect`)

(fn `ResetEffectOnBeat`
  (if (`/Game/Blueprints/BeatChecker.bOnBeat` (`self.BeatChecker`))
    (`self.ResetEffect`)
    (else
      (`KismetSystemLibrary.K2_SetTimer` null "ResetEffectOnBeat" 0.05))))

(fn `ResetExit`
  (bind _exit (`self.Exit`))
  (`PrimitiveComponent.SetCollisionEnabled` (`/Game/Blueprints/BP_GargantuaLogic.Center` _exit) "QueryAndPhysics")
  (`PrimitiveComponent.SetCollisionEnabled` (`/Game/Blueprints/BP_GargantuaLogic.Outer` _exit) "QueryAndPhysics")
  (set `/Game/Blueprints/BP_GargantuaLogic.BlackHoleOn` false _exit)
  (set `/Game/Blueprints/BP_GargantuaLogic.IsExit` false _exit))

(fn `SetExit`
  (bind _exit (`self.Exit`))
  (`PrimitiveComponent.SetCollisionEnabled` (`/Game/Blueprints/BP_GargantuaLogic.Center` _exit) "NoCollision")
  (`PrimitiveComponent.SetCollisionEnabled` (`/Game/Blueprints/BP_GargantuaLogic.Outer` _exit) "NoCollision")
  (set `/Game/Blueprints/BP_GargantuaLogic.IsExit` true _exit))

(fn `SetLocationToExit`
  (params (BoxCharacter :type "Actor Object Reference") (Exit :type "Actor Object Reference"))
  (`self.K2_SetActorLocation` BoxCharacter (`self.K2_GetActorLocation` Exit) false true)
  (return))

(fn `UserConstructionScript`
  (locals (NewLocalVar :type "Vector Structure" :default (0.0 0.0 0.0))))