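; BP_Sentinel is a roaming, spinning enemy that attacks players in time with the music via BeatChecker.
; Req/Res event pairs drive a delayed shockwave, which moves it on a timeline and triggers the BP_WavyFloor below, and lasers aimed at the closest pawn from the nearest of four attached emitters.
; Tick chains server work into multicast motion, tracks pawn distances and pulls physics boxes toward its AntiGravityField with inverse-square force.
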(event `self.ReceiveBeginPlay`
  ;[1 1 1] BeginPlay
  (`|ExecutionSequence`
    (:`then_0`
      (set `self.StartPos` (`self.K2_GetActorLocation`))
      (`KismetSystemLibrary.K2_SetTimer` null "StartBasicLaserOnBeat" 5.0)
      (`KismetSystemLibrary.Delay` 30.0)
      (`self.ShockWaveOnBeat`))
    (:`then_1`
      (`KismetSystemLibrary.K2_SetTimerForNextTick` null "SetBeatLength"))
    (:`then_2`
      (`/Engine/EditorBlueprintResources/ActorMacros.Switch Has Authority`
        (:`Authority`
          (`KismetSystemLibrary.K2_SetTimerForNextTick` null "EnlistPlayers"))))))

(event `self.ReceiveTick`
  (params (DeltaSeconds :type "Float (single-precision)"))
  ;[1 1 1] Tick
  (`self.TickOnServer` DeltaSeconds))

(event `TickOnServer`
  (params (DeltaSeconds :type "Float (double-precision)"))
  ;[1 1 1] Tick
  (`self.TickMultiCast` DeltaSeconds)
  (`self.AntiGravity`)
  (`self.CheckPlayerDistances`))

(event `TickMultiCast`
  (params (DeltaSeconds :type "Float (double-precision)"))
  ;[1 1 1] Tick
  (`self.Roaming` DeltaSeconds)
  (`self.ComponentsRotation`)
  (`self.UpdateLaserLocations`))

(event `ReqShockWave`
  ;[1 1 1] ShockWave
  (`self.ResShockWave`))

(event `ResShockWave`
  (bind (_current_pos_x _current_pos_y _current_pos_z) (`KismetMathLibrary.BreakVector` (`self.Current_Pos`)))
  (bind (_current_rot_roll _current_rot_pitch _current_rot_yaw) (`KismetMathLibrary.BreakRotator` (`self.Current_Rot`)))
  ;[1 1 1] ShockWave
  (set `self.moving` false)
  (set `self.Current_Pos` (`self.K2_GetActorLocation`))
  (set `self.Current_Rot` (`self.K2_GetActorRotation`))
  (`|ExecutionSequence`
    (:`then_0`
      (bind (_direction _skill _rotate_rate) (`Timeline|ShockWave_Movement` :!via `PlayFromStart`)
        (:`Update`
          (`self.K2_SetActorLocation` (`KismetMathLibrary.MakeVector` _current_pos_x _current_pos_y (+ _current_pos_z (* _skill 350.0))))
          (`self.K2_SetActorRotation` (`KismetMathLibrary.MakeRotator` 0.0 0.0 (+ (* _rotate_rate -100.0) _current_rot_yaw))))
        (:`Finished`
          ;;[1 0.2448 0.2448] Fin
          (set `self.moving` true))))
    (:`then_1`
      (`KismetSystemLibrary.K2_SetTimer` null "TriggerWavyFloor" (* 2.0 (`self.BeatLength`))))))

(event `ReqBasicLaser`
  ;[1 1 1] BasicLaser
  (bind _closestplayerindex (`self.WhoIsTheClosest?`))
  (bind _output (`|GetArrayItem` (`self.Players`) _closestplayerindex))
  (bind _closestlaserindex (`self.WhichLaserIsTheClosest?` (`self.K2_GetActorLocation` _output)))
  (bind _output_2 (`|GetArrayItem` (`self.Lasers`) _closestlaserindex))
  (if (not (`/Game/Blueprints/BP_Beam.bLaserTrigger` _output_2))
    (`self.ResBasicLaser` _output_2 _output)))

(event `ResBasicLaser`
  (params (`타깃` :type "/Game/Blueprints/BP_Beam Object Reference") (AimTarget :type "Actor Object Reference"))
  ;[1 1 1] BasicLaser
  (`/Game/Blueprints/BP_Beam.Ready` `타깃` AimTarget))

(fn `AntiGravity`
  (for _array_element (`PrimitiveComponent.GetOverlappingActors` (`self.AntiGravityField`) "/Game/GameMode/BP_CBox.BP_CBox_C")
    (bind _asbp_cbox (cast `/Game/GameMode/BP_CBox` _array_element))
    (bind _returnvalue (- (`SceneComponent.K2_GetComponentLocation` (`self.AntiGravityField`)) (`self.K2_GetActorLocation` _asbp_cbox)))
    (`PrimitiveComponent.SetPhysicsLinearVelocity` (`BoxCharacter.Cube` _asbp_cbox) (/ (* (`KismetMathLibrary.Normal` _returnvalue) (`self.Gravity`)) (`KismetMathLibrary.VSizeSquared` _returnvalue)) true "None")))

(fn `CheckPlayerDistances`
  (for (_array_element _array_index) (`self.Players`)
    (`KismetArrayLibrary.Array_Set` (`self.PlayerDistances`) _array_index (`KismetMathLibrary.VSize` (- (`self.K2_GetActorLocation` _array_element) (`self.K2_GetActorLocation`))))))

(fn `ComponentsRotation`
  (bind _timer (`self.Timer`))
  (`SceneComponent.K2_SetWorldRotation` (`self.core`) (`KismetMathLibrary.MakeRotator` (* _timer 144.0) (* _timer 26.0) (* _timer 99.0)) false false)
  (`SceneComponent.K2_SetWorldRotation` (`self.Halo`) (`KismetMathLibrary.MakeRotator` 0.0 0.0 (* -33.0 (`self.Timer`))) false false))

(fn `EnlistPlayers`
  (`KismetArrayLibrary.Array_Clear` (`self.PlayerDistances`))
  (bind _outactors (`GameplayStatics.GetAllActorsOfClass` "/Script/Engine.Pawn"))
  (bind _output_get (set `self.Players` _outactors))
  (for _ _output_get
    (`KismetArrayLibrary.Array_Add` (`self.PlayerDistances`))))

(fn `Roaming`
  (params (DeltaSeconds :type "Float (double-precision)"))
  (bind _width_value (`self.width Value`))
  (bind _returnvalue (* (`self.Timer4Movement`) (`self.Speed (horizental)`)))
  ;[1 1 1] Timers
  (set `self.Timer` (+ (`self.Timer`) DeltaSeconds))
  (if (`self.moving`)
    (set `self.Timer4Movement` (+ (`self.Timer4Movement`) DeltaSeconds))
    ;[1 1 1] Location
    (`self.K2_SetActorLocation` (+ (`self.StartPos`) (`KismetMathLibrary.MakeVector` (* (* 1.0 (`KismetMathLibrary.Sin` (* _returnvalue 1.7))) _width_value) (* _width_value (* (`KismetMathLibrary.Cos` (* _returnvalue 1.0)) 3.0)) (* (`KismetMathLibrary.Sin` (* (* (`self.Timer4Movement`) (`self.Speed (vertical)`)) 20.0)) (`self.heigth Value`)))))
    ;[1 1 1] Rotation
    (`self.K2_SetActorRotation` (`KismetMathLibrary.MakeRotator` 0.0 0.0 (* (`self.Timer4Movement`) (`self.ActorRotSpeed`))))))

(fn `SetArrowRot`
  (params (`타깃` :type "SceneComponent Object Reference"))
  (`SceneComponent.K2_SetWorldRotation` `타깃` (`KismetMathLibrary.FindLookAtRotation` (`SceneComponent.K2_GetComponentLocation` `타깃`) (`SceneComponent.K2_GetComponentLocation` (`Actor.RootComponent` (`GameplayStatics.GetPlayerPawn` 0)))) false false))

(fn `SetBeatLength`
  (bind _output_get (set `self.BeatLength` (`/Game/Blueprints/CPNT_BeatChecker.BeatLength` (`self.BeatChecker`))))
  (`FXSystemComponent.SetFloatParameter` (`self.AudioReactiveParticles`) "BeatLength" _output_get)
  (`TimelineComponent.SetPlayRate` (`self.ShockWave_Movement`) (/ 1.0 (* 8.0 (`self.BeatLength`)))))

(fn `ShockWaveOnBeat`
  (if (`/Game/Blueprints/CPNT_BeatChecker.bOnBeat` (`self.BeatChecker`))
    (`self.ReqShockWave`)
    (else
      (`KismetSystemLibrary.K2_SetTimer` null "ShockWaveOnBeat" 0.03))))

(fn `StartBasicLaserOnBeat`
  (if (`/Game/Blueprints/CPNT_BeatChecker.bOnBeat` (`self.BeatChecker`))
    (bind _returnvalue (`KismetSystemLibrary.K2_SetTimerDelegate` (`|CreateDelegate` :!event `ReqBasicLaser`) (`self.BeatLength`) true))
    (set `self.BasicLaserHandler` _returnvalue)
    (else
      (`KismetSystemLibrary.K2_SetTimer` null "BasicLaserOnBeat" 0.03))))

(fn `TriggerWavyFloor`
  (bind _ng_shockwaveimpact (`self.NG_ShockWaveImpact`))
  (bind _outhit (`KismetSystemLibrary.LineTraceSingleByProfile` (`self.K2_GetActorLocation`) (+ (`self.K2_GetActorLocation`) (0.0 0.0 -33333.0))))
  (bind _asbp_wavy_floor (cast `/Game/Blueprints/BP_WavyFloor` (`.HitActor` (`GameplayStatics.BreakHitResult` _outhit))))
  (`/Game/Blueprints/BP_WavyFloor.Trigger` _asbp_wavy_floor false 0.0)
  (`SceneComponent.K2_SetWorldLocation` _ng_shockwaveimpact (+ (`.Location` (`GameplayStatics.BreakHitResult` _outhit)) (0.0 0.0 111.0)) false false)
  (`NiagaraComponent.ResetSystem` _ng_shockwaveimpact))

(fn `UpdateLaserLocations`
  (`self.K2_SetActorLocation` (`|GetArrayItem` (`self.Lasers`)) (`SceneComponent.K2_GetComponentLocation` (`self.Arrow1`)) false false)
  (`self.K2_SetActorLocation` (`|GetArrayItem` (`self.Lasers`) 1) (`SceneComponent.K2_GetComponentLocation` (`self.Arrow2`)) false false)
  (`self.K2_SetActorLocation` (`|GetArrayItem` (`self.Lasers`) 2) (`SceneComponent.K2_GetComponentLocation` (`self.Arrow3`)) false false)
  (`self.K2_SetActorLocation` (`|GetArrayItem` (`self.Lasers`) 3) (`SceneComponent.K2_GetComponentLocation` (`self.Arrow4`)) false false))

(fn `UserConstructionScript`)

(fn `WhichLaserIsTheClosest?`
  (params (TargetLocation :type "Vector Structure"))
  (returns (ClosestLaserIndex :type Integer))
  (locals (ClosestDistance :type "Float (double-precision)" :default 999999999999999.0) (Index :type Integer))
  (for (_array_element _array_index) (`self.Lasers`)
    (bind _returnvalue (`KismetMathLibrary.VSizeSquared` (- (`self.K2_GetActorLocation` _array_element) TargetLocation)))
    (if (> (`local.ClosestDistance`) _returnvalue)
      (set `local.ClosestDistance` _returnvalue)
      (set `local.Index` _array_index)))
  (return (`local.Index`)))

(fn `WhoIsTheClosest?`
  (returns (ClosestPlayerIndex :type Integer))
  (locals (ClosestDistance :type "Float (double-precision)" :default 999999999999999.0) (Index :type Integer))
  (set `local.ClosestDistance` 999999999999999.0)
  (for (_array_element _array_index) (`self.PlayerDistances`)
    (if (> (`local.ClosestDistance`) _array_element)
      (set `local.ClosestDistance` _array_element)
      (set `local.Index` _array_index)))
  (return (`local.Index`)))