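; CPNT_BeatChecker is a component that gives its owner a local copy of the game's beat state.
; On BeginPlay it waits a zero-length delay, then caches BP_MyGameState and copies its BeatLength once.
; It binds to the game state's SetOnBeat event dispatcher and refreshes its own OnBeat value each time that fires, so it needs no polling.
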(event `self.ReceiveBeginPlay`
  (`KismetSystemLibrary.Delay` 0.0)
  (bind _asbp_my_game_state (cast `/Game/GameMode/BP_MyGameState` (`GameplayStatics.GetGameState`)))
  (bind _output_get (set `self.MyGameState` _asbp_my_game_state))
  (set `self.BeatLength` (`/Game/GameMode/BP_MyGameState.BeatLength` _output_get))
  (add `/Game/GameMode/BP_MyGameState.EVDSPC_SetOnBeat` (`self.MyGameState`) (delegate `EV_SetOnBeat`)))

(event `EV_SetOnBeat`
  (set `self.bOnBeat` (`/Game/GameMode/BP_MyGameState.OnBeat` (`self.MyGameState`))))