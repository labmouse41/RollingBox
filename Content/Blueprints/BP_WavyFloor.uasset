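; BP_WavyFloor is a floor tile that passes a vertical wave to neighboring tiles when triggered.
; Shortly after BeginPlay it caches overlapping tiles as neighbors and feeds BeatLength to its mesh material.
; Trigger runs a timeline driving world Z and recursively triggers neighbors with small random delays, while a Triggered flag blocks re-entry until the motion finishes.
; Enlist2Holder can register the tile with BP_WavyFloorHolder.
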(event `self.ReceiveBeginPlay`
  (`KismetSystemLibrary.K2_SetTimer` null "Initialize" 0.1))

(event `Trigger`
  (params (Delay :type Boolean) (DelayTime :type "Float (double-precision)"))
  ;[1 1 1] Trigger
  (if (not (`self.bTriggered`))
    (set `self.bTriggered` true)
    (`KismetSystemLibrary.Delay` (* (`KismetMathLibrary.Conv_BoolToDouble` Delay) DelayTime))
    (`|ExecutionSequence`
      (:`then_0`
        (`self.AfterTrigger`))
      (:`then_1`
        (for _array_element (`self.NeighborList`)
          (`self.Trigger` _array_element true (`KismetMathLibrary.RandomFloatInRange` 0.05 0.1)))))))

(event `AfterTrigger`
  (bind (_returnvalue_x _returnvalue_y) (`KismetMathLibrary.BreakVector` (`self.K2_GetActorLocation`)))
  ;[1 1 1] Trigger
  (bind (_direction `_새_트랙_0`) (`Timeline|posZ` :!via `PlayFromStart`)
    (:`Update`
      (`self.K2_SetActorLocation` (`KismetMathLibrary.MakeVector` _returnvalue_x _returnvalue_y (* (- 1.0 `_새_트랙_0`) 111.0))))
    (:`Finished`
      ;;[1 0.184 0.184] Fin
      (set `self.bTriggered` false))))

(fn `Enlist2Holder`
  (bind _returnvalue (`GameplayStatics.GetActorOfClass` "/Game/Blueprints/BP_WavyFloorHolder.BP_WavyFloorHolder_C"))
  (`KismetArrayLibrary.Array_Add` (`/Game/Blueprints/BP_WavyFloorHolder.List` _returnvalue) self)
  (set `self.BeatLength` (`/Game/Blueprints/BeatChecker.BeatLength` (`/Game/Blueprints/BP_WavyFloorHolder.BeatChecker` _returnvalue))))

(fn `Initialize`
  (for _array_element (`PrimitiveComponent.GetOverlappingActors` (`self.NeighborDetector`) "BP_WavyFloor_C")
    (bind _asbp_wavy_floor (cast `/Game/Blueprints/BP_WavyFloor` _array_element))
    (`KismetArrayLibrary.Array_Add` (`self.NeighborList`) _asbp_wavy_floor)
    (`KismetArrayLibrary.Array_RemoveItem` (`self.NeighborList`) self)
    (`MeshComponent.SetScalarParameterValueOnMaterials` (`self.StaticMesh`) "BeatLength" (`/Game/Blueprints/BeatChecker.BeatLength` (`self.BeatChecker`)))))

(fn `UserConstructionScript`)