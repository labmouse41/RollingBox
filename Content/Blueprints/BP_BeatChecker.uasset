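; BP_BeatChecker is a Blueprint that visualizes a beat by scaling a cube.
; BeginPlay starts a non-looping timer that calls BeatHit after BeatLength seconds and sets the timeline's play rate to the inverse of BeatLength.
; BeatHit plays the timeline, whose track value plus one drives the cube's uniform world scale on each update.
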(event `self.ReceiveBeginPlay`
  (`KismetSystemLibrary.K2_SetTimerDelegate` (delegate `BeatHit`) (`self.BeatLength`))
  (`TimelineComponent.SetPlayRate` (`self.타임라인`) (/ 1.0 (`self.BeatLength`))))

(event `BeatHit`
  (bind (_direction `_새_트랙_0`) (`Timeline|타임라인`)
    (:`Update`
      (`SceneComponent.SetWorldScale3D` (`self.Cube`) (`KismetMathLibrary.Conv_DoubleToVector` (+ `_새_트랙_0` 1.0))))))

(fn `UserConstructionScript`)