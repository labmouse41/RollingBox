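; Black hole teleporter that pulls in a box character and flings it out of another black hole.
; On BeginPlay, the authority picks a random other BP_CubicBlackHole as a fixed exit.
; Overlap starts a burst effect on both ends, disables the exit's collision, and Tick pulls the character's cube inward.
; A timed Release moves the character to the exit, launches it in a random direction, then shortly re-enables the exit.
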(event `self.ReceiveBeginPlay`
  (`/Engine/EditorBlueprintResources/ActorMacros.Switch Has Authority`
    (:`Authority`
      (bind _outactors (`GameplayStatics.GetAllActorsOfClass` "BP_CubicBlackHole_C"))
      (bind _output_get (set `self.BlackHoleList` _outactors))
      (`KismetArrayLibrary.Array_RemoveItem` _output_get self)
      (set `self.Exit` (`KismetArrayLibrary.Array_Random` (`self.BlackHoleList`))))))

(event `self.ReceiveTick`
  (params (DeltaSeconds :type "Float (single-precision)"))
  (bind _targetcharacter (`self.TargetCharacter`))
  (if (`self.BlackHoleOn`)
    (`PrimitiveComponent.SetPhysicsLinearVelocity` (`/Game/GameMode/BP_Boxcharacter.Cube` _targetcharacter) (* (`KismetMathLibrary.Normal` (- (`self.K2_GetActorLocation`) (`self.K2_GetActorLocation` _targetcharacter))) (`self.Gravity`) (`GameplayStatics.GetWorldDeltaSeconds`)) true "None")))

(event `PlayEffect`
  (`FXSystemComponent.SetFloatParameter` (`self.PortalCore`) "GravityMultiplier" 222.0)
  (`FXSystemComponent.SetFloatParameter` (`self.PortalParticles`) "GravityMultiplier" 222.0)
  (`MeshComponent.SetScalarParameterValueOnMaterials` (`self.InnerRefraction`) "TimeSpeed" 9.0)
  (`SceneComponent.SetRelativeScale3D` (`self.InnerRefraction`) (0.4 0.4 0.4))
  (`KismetSystemLibrary.K2_SetTimer` null "ResetEffect" 1.0))

(event `self.Box.OnComponentBeginOverlap`
  (params (OverlappedComponent :type "PrimitiveComponent Object Reference") (OtherActor :type "Actor Object Reference") (OtherComp :type "PrimitiveComponent Object Reference") (OtherBodyIndex :type Integer) (bFromSweep :type Boolean) (SweepResult :type "HitResult Structure (by ref)"))
  (if (`self.IsExit`)
    _
    (elif (not (`self.BlackHoleOn`))
      (bind _asbp_boxcharacter (cast `/Game/GameMode/BP_Boxcharacter` OtherActor))
      (set `self.TargetCharacter` _asbp_boxcharacter)
      (`self.PlayEffect`)
      (set `self.BlackHoleOn` true)
      (`self.SetExit`)
      (`KismetSystemLibrary.K2_SetTimer` null "Release" 1.0))))

(fn `Release`
  (`self.SetLocationToExit` (`self.TargetCharacter`) (`self.Exit`))
  (`PrimitiveComponent.SetPhysicsLinearVelocity` (`/Game/GameMode/BP_Boxcharacter.Cube` (`self.TargetCharacter`)) (* (`KismetMathLibrary.RandomUnitVector`) (`self.OutPower`)) false "None")
  (set `self.BlackHoleOn` false)
  (`KismetSystemLibrary.K2_SetTimer` null "ResetExit" 0.1))

(fn `ResetEffect`
  (`FXSystemComponent.SetFloatParameter` (`self.PortalCore`) "GravityMultiplier" 1.0)
  (`FXSystemComponent.SetFloatParameter` (`self.PortalParticles`) "GravityMultiplier" 1.0)
  (`MeshComponent.SetScalarParameterValueOnMaterials` (`self.InnerRefraction`) "TimeSpeed" 0.7)
  (`SceneComponent.SetRelativeScale3D` (`self.InnerRefraction`) (0.5 0.5 0.5))
  (`SceneComponent.SetVisibility` (`self.OuterRefraction`) true false))

(fn `ResetExit`
  (bind _exit (`self.Exit`))
  (`PrimitiveComponent.SetCollisionEnabled` (`/Game/Blueprints/BP_CubicBlackHole.Box` _exit) "QueryAndPhysics")
  (set `/Game/Blueprints/BP_CubicBlackHole.BlackHoleOn` false _exit)
  (set `/Game/Blueprints/BP_CubicBlackHole.IsExit` false _exit))

(fn `SetExit`
  (bind _exit (`self.Exit`))
  (`PrimitiveComponent.SetCollisionEnabled` (`/Game/Blueprints/BP_CubicBlackHole.Box` _exit) "NoCollision")
  (set `/Game/Blueprints/BP_CubicBlackHole.IsExit` true _exit)
  (`self.PlayEffect` _exit))

(fn `SetLocationToExit`
  (params (BoxCharacter :type "Actor Object Reference") (Exit :type "Actor Object Reference"))
  (`self.K2_SetActorLocation` BoxCharacter (`self.K2_GetActorLocation` Exit) false false)
  (return))

(fn `UserConstructionScript`
  (locals (NewLocalVar :type "Vector Structure" :default (0.0 0.0 0.0))))