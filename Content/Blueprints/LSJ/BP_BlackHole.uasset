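; BP_BlackHole is a teleporting black hole that pulls in BP_Boxcharacter and flings it out at another black hole.
; Overlapping its ErgoSphere disables the box's gravity and starts a per-Tick pull, then a one-second delay precedes teleport and random launch.
; IsExit and disabled collision aim to prevent recapture until end overlap resets them.
; Random is re-evaluated per use, so flagged, destination and collision-disabled holes can differ.
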(event `self.ReceiveBeginPlay`
  (`|ExecutionSequence`
    (:`then_0`
      (bind _outactors (`GameplayStatics.GetAllActorsOfClass` "BP_BlackHole_C"))
      (bind _output_get (set `self.BlackHoleList` _outactors))
      (`KismetArrayLibrary.Array_RemoveItem` _output_get self))))

(event `self.ReceiveTick`
  (params (DeltaSeconds :type "Float (single-precision)"))
  ;[1 1 1] ErgoSphere
  (if (`self.BlackHoleOn`)
    (for _array_element (`PrimitiveComponent.GetOverlappingActors` (`self.ErgoSphere`) "/Game/GameMode/BP_Boxcharacter.BP_Boxcharacter_C")
      (bind _asbp_boxcharacter (cast `/Game/GameMode/BP_Boxcharacter` _array_element))
      (`PrimitiveComponent.SetPhysicsLinearVelocity` (`/Game/GameMode/BP_Boxcharacter.Cube` _asbp_boxcharacter) (* (`KismetMathLibrary.Normal` (- (`self.K2_GetActorLocation`) (`self.K2_GetActorLocation` _array_element))) (`self.Gravity`)) true "None"))))

(event `self.ErgoSphere.OnComponentBeginOverlap`
  (params (OverlappedComponent :type "PrimitiveComponent Object Reference") (OtherActor :type "Actor Object Reference") (OtherComp :type "PrimitiveComponent Object Reference") (OtherBodyIndex :type Integer) (bFromSweep :type Boolean) (SweepResult :type "HitResult Structure (by ref)"))
  (bind (_returnvalue_x _returnvalue_y) (`KismetMathLibrary.BreakVector` (`KismetMathLibrary.RandomUnitVector`)))
  ;[1 1 1] ErgoSphere
  (if (not (`self.IsExit`))
    (bind _asbp_boxcharacter (cast `/Game/GameMode/BP_Boxcharacter` OtherActor))
    (bind _cube (`/Game/GameMode/BP_Boxcharacter.Cube` _asbp_boxcharacter))
    (`PrimitiveComponent.SetEnableGravity` _cube false)
    (set `self.BlackHoleOn` true)
    (`KismetSystemLibrary.Delay` 1.0)
    (bind _exit (`self.Set New Location` OtherActor))
    (`PrimitiveComponent.SetCollisionEnabled` (`/Game/Blueprints/LSJ/BP_BlackHole.ErgoSphere` _exit) "NoCollision")
    (`PrimitiveComponent.SetPhysicsLinearVelocity` _cube (* (+ _returnvalue_x _returnvalue_y 1.0) (`self.OutPower`)) false "None")))

(event `self.ErgoSphere.OnComponentEndOverlap`
  (params (OverlappedComponent :type "PrimitiveComponent Object Reference") (OtherActor :type "Actor Object Reference") (OtherComp :type "PrimitiveComponent Object Reference") (OtherBodyIndex :type Integer))
  ;[1 1 1] ErgoSphere
  (bind _asbp_boxcharacter (cast `/Game/GameMode/BP_Boxcharacter` OtherActor))
  (`PrimitiveComponent.SetEnableGravity` (`/Game/GameMode/BP_Boxcharacter.Cube` _asbp_boxcharacter) true)
  (`PrimitiveComponent.SetCollisionEnabled` (`self.ErgoSphere`) "QueryAndPhysics")
  (set `self.BlackHoleOn` false)
  (set `self.IsExit` false))

(fn `Set New Location`
  (params (`타깃` :type "Actor Object Reference"))
  (returns (Exit :type "/Game/Blueprints/LSJ/BP_BlackHole Object Reference"))
  (bind _outitem (`KismetArrayLibrary.Array_Random` (`self.BlackHoleList`)))
  (set `/Game/Blueprints/LSJ/BP_BlackHole.IsExit` true _outitem)
  (`SceneComponent.K2_SetRelativeLocation` (`Actor.RootComponent` `타깃`) (`self.K2_GetActorLocation` _outitem) false false)
  (return _outitem))

(fn `UserConstructionScript`
  (locals (NewLocalVar :type "Vector Structure" :default (0.0 0.0 0.0))))