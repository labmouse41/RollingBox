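; BP_LaserSpawner is an actor that spawns a laser in time with the game's beat.
; Each tick it checks OnBeat on BP_MyGameMode and its own Trigger flag, then spawns the class that LaserType selects from the Class array.
; The spawn uses the StaticMesh component's relative transform.
; Trigger clears after each spawn, and nothing in this graph sets it again.
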(event `self.ReceiveTick`
  (params (DeltaSeconds :type "Float (single-precision)"))
  (if (and (`/Game/GameMode/BP_MyGameMode.bOnBeat` (cast `/Game/GameMode/BP_MyGameMode` (`GameplayStatics.GetGameMode`) :!pure true)) (`self.Trigger`))
    (`|SpawnActorFromClass` (`|GetArrayItem` (`self.Class`) (`self.LaserType`)) (`SceneComponent.GetRelativeTransform` (`self.StaticMesh`)) "Undefined" "OverrideRootScale" null null)
    (set `self.Trigger` false)))

(fn `UserConstructionScript`)