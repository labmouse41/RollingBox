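; BP_Laser is a laser hazard that telegraphs with a guide line, then fires and launches box characters on contact.
; BeginPlay sets the GuideLine scale and starts a three-second timer that calls Bim by name to scale up the Cylinder beam.
; Cylinder hits on a BP_Boxcharacter overwrite its Cube's physics velocity with Power, aimed toward a point offset from the laser's location.
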(event `self.ReceiveBeginPlay`
  (`SceneComponent.K2_SetRelativeTransform` (`self.GuideLine`) (`KismetMathLibrary.MakeTransform` (0.0 0.0 0.0) (struct) (0.1 0.1 10.0)) false false)
  (`KismetSystemLibrary.K2_SetTimer` null "Bim" 3.0))

(event `self.Cylinder.OnComponentHit`
  (params (HitComponent :type "PrimitiveComponent Object Reference") (OtherActor :type "Actor Object Reference") (OtherComp :type "PrimitiveComponent Object Reference") (NormalImpulse :type "Vector Structure") (Hit :type "HitResult Structure (by ref)"))
  (bind _asbp_boxcharacter (cast `/Game/GameMode/BP_Boxcharacter` OtherActor))
  (`PrimitiveComponent.SetPhysicsLinearVelocity` (`/Game/GameMode/BP_Boxcharacter.Cube` _asbp_boxcharacter) (* (`KismetMathLibrary.GreaterGreater_VectorRotator` (`KismetMathLibrary.GetForwardVector` (`KismetMathLibrary.FindLookAtRotation` (`self.K2_GetActorLocation` OtherActor) (+ (`self.K2_GetActorLocation`) 500.0))) (struct)) (`self.Power`)) false "None"))

(fn `Bim`
  (`SceneComponent.K2_SetRelativeTransform` (`self.Cylinder`) (`KismetMathLibrary.MakeTransform` (0.0 0.0 0.0) (struct) (0.5 0.5 10.0)) false false))

(fn `UserConstructionScript`)