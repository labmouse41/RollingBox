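; BP_Trampline is a trampoline actor that pulses to the game's beat and launches whatever touches it.
; A looping timer at BP_MyGameMode's BeatLength restarts a timeline whose play rate is the inverse of that length.
; The timeline track swells the scale of Box0 on each beat.
; Overlapping the box replaces the other component's physics velocity with a fixed speed along the Arrow's forward vector, independent of the pulse.
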(event `self.ReceiveBeginPlay`
  (bind _beatlength (`/Game/GameMode/BP_MyGameMode.BeatLength` (cast `/Game/GameMode/BP_MyGameMode` (`GameplayStatics.GetGameMode`) :!pure true)))
  (`TimelineComponent.SetPlayRate` (`self.타임라인`) (/ 1.0 _beatlength))
  (`KismetSystemLibrary.K2_SetTimerDelegate` (delegate `TramPoline`) _beatlength true))

(event `TramPoline`
  (bind (_direction `_새_트랙_0`) (`Timeline|타임라인` :!via `PlayFromStart`)
    (:`Update`
      (bind _returnvalue (* `_새_트랙_0` 0.5))
      (`SceneComponent.SetWorldScale3D` (`self.Box_0`) (`KismetMathLibrary.MakeVector` (+ _returnvalue 2.0) (+ _returnvalue 2.0) (+ _returnvalue 0.5))))))

(event `self.Box_0.OnComponentBeginOverlap`
  (params (OverlappedComponent :type "PrimitiveComponent Object Reference") (OtherActor :type "Actor Object Reference") (OtherComp :type "PrimitiveComponent Object Reference") (OtherBodyIndex :type Integer) (bFromSweep :type Boolean) (SweepResult :type "HitResult Structure (by ref)"))
  (`PrimitiveComponent.SetPhysicsLinearVelocity` OtherComp (* (`SceneComponent.GetForwardVector` (`self.Arrow`)) 1000.0) false "None"))

(fn `UserConstructionScript`
  (`parent.UserConstructionScript`))