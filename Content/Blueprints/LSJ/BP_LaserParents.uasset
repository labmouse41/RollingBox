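; Base laser hazard actor that stretches a guide line to LaserLength and knocks back what touches its laser mesh.
; Tick counts frames and calls Beam every 30th, so timing depends on frame rate; Beam is empty here.
; On mesh overlap, Overlap disables the other actor's input and sets its component's physics velocity from the laser-to-component look-at rotation scaled by Power.
; Nothing here re-enables input.
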(event `self.ReceiveBeginPlay`
  (`SceneComponent.K2_SetRelativeTransform` (`self.GuideLineScene`) (`KismetMathLibrary.MakeTransform` (0.0 0.0 0.0) (struct) (`KismetMathLibrary.MakeVector` 1.0 1.0 (`self.LaserLength`))) false false))

(event `self.ReceiveTick`
  (params (DeltaSeconds :type "Float (single-precision)"))
  (if true
    (set `self.set_Count` (+ (`self.set_Count`) 1))
    (if (== (`self.set_Count`) 30)
      (`self.Beam`)
      (set `self.set_Count` 0))))

(event `Beam`)

(event `self.LaserMesh.OnComponentBeginOverlap`
  (params (OverlappedComponent :type "PrimitiveComponent Object Reference") (OtherActor :type "Actor Object Reference") (OtherComp :type "PrimitiveComponent Object Reference") (OtherBodyIndex :type Integer) (bFromSweep :type Boolean) (SweepResult :type "HitResult Structure (by ref)"))
  (`self.Overlap` OtherComp OverlappedComponent OtherActor OtherComp))

(fn `Overlap`
  (params (StartLocationTarget :type "SceneComponent Object Reference") (TargetLocationTarget :type "SceneComponent Object Reference") (DisableInputTarget :type "Actor Object Reference") (PhysicsVelocityTarget :type "PrimitiveComponent Object Reference"))
  (`self.DisableInput` DisableInputTarget (`GameplayStatics.GetPlayerController` 0))
  (`PrimitiveComponent.SetPhysicsLinearVelocity` PhysicsVelocityTarget (* (`KismetMathLibrary.FindLookAtRotation` (`SceneComponent.K2_GetComponentLocation` TargetLocationTarget) (`SceneComponent.K2_GetComponentLocation` StartLocationTarget)) (`self.Power`)) false "None"))

(fn `UserConstructionScript`)