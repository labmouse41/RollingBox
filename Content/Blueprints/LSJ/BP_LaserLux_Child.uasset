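; BP_LaserLux_Child is a child laser Blueprint that overrides the Beam event to animate a one-shot beam.
; Beam hides the guide line mesh, then a timeline stretches LaserScene along Z up to LaserLength.
; A second timeline then animates the beam's X/Y thickness, re-enabling player 0's pawn input on each update, and destroys the actor when finished.
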(event `self.Beam`
  (`SceneComponent.SetHiddenInGame` (`self.GuideLineMesh`) true false)
  (bind (_direction `_새_트랙_0`) (`Timeline|타임라인`)
    (:`Update`
      (`SceneComponent.K2_SetRelativeTransform` (`self.LaserScene`) (`KismetMathLibrary.MakeTransform` (0.0 0.0 0.0) (struct) (`KismetMathLibrary.MakeVector` 0.5 0.5 (`KismetMathLibrary.Lerp` 0.0 (`self.LaserLength`) `_새_트랙_0`))) false false))
    (:`Finished`
      (bind (_direction_2 `_새_트랙_0_2`) (`Timeline|타임라인_0` :!via `PlayFromStart`)
        (:`Update`
          (`self.EnableInput` (`GameplayStatics.GetPlayerPawn` 0) (`GameplayStatics.GetPlayerController` 0))
          (bind _returnvalue (`KismetMathLibrary.Lerp` 0.0 0.5 `_새_트랙_0_2`))
          (`SceneComponent.K2_SetRelativeTransform` (`self.LaserScene`) (`KismetMathLibrary.MakeTransform` (0.0 0.0 0.0) (struct) (`KismetMathLibrary.MakeVector` _returnvalue _returnvalue (`self.LaserLength`))) false false))
        (:`Finished`
          (`self.K2_DestroyActor`))))))

(fn `UserConstructionScript`
  (`parent.UserConstructionScript`))